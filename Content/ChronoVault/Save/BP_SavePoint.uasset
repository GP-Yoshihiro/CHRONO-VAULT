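; BP_SavePoint is a save point that records the player's respawn transform when the player overlaps its capsule.
; A one-second delay after BeginPlay arms it, preventing an immediate re-save right after respawn.
; On overlap it uses BPI_Player messages instead of casts to trigger a green screen flash and save the Arrow's world transform, including facing, alongside a save sound.
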(event `self.ReceiveBeginPlay`
  ;[0.05 0.25 0.4 0.6] 復活直後に再セーブしないよう少し待つ
  (`KismetSystemLibrary.Delay` 1.0)
  (set `self.bReady` true))

(event `self.Capsule.OnComponentBeginOverlap`
  (params (OverlappedComponent :type "PrimitiveComponent Object Reference") (OtherActor :type "Actor Object Reference") (OtherComp :type "PrimitiveComponent Object Reference") (OtherBodyIndex :type Integer) (bFromSweep :type Boolean) (SweepResult :type "HitResult Structure (by ref)"))
  ;[0.1 0.35 0.15 0.6] 接触：画面フラッシュ → Arrowの向きを含むTransformを保存（BPI_Player経由・Castなし）
  (if (and (`KismetSystemLibrary.DoesImplementInterface` OtherActor "/Game/ChronoVault/Player/BPI_Player.BPI_Player_C") (`self.bReady`))
    (message `/Game/ChronoVault/Player/BPI_Player.PlayerPlayScreenEffect` OtherActor (struct :`R` 0.05 :`G` 1.0 :`B` 0.3 :`A` 1.0))
    (`GameplayStatics.PlaySound2D` "/Game/ChronoVault/Audio/SE/SE_Save.SE_Save" 1.0 1.0 0.0 null null)
    (message `/Game/ChronoVault/Player/BPI_Player.PlayerSaveData` OtherActor (`SceneComponent.K2_GetComponentToWorld` (`self.Arrow`)))))

(fn `UserConstructionScript`)