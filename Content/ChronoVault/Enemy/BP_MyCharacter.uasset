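; Enemy character Blueprint that patrols, chases when alerted and melee-attacks players inside its AttackSphere.
; Overlapping a BPI_Player actor starts a looping TryAttack timer, which plays a dynamic montage and applies damage after a delay if the target remains.
; SetDiscovered switches walk speed, eye light color, sound and the overhead UW_Alert mark.
; GetNextPatrolPoint cycles through PatrolPoints; neither function is called within this Blueprint.
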(event `TryAttack`
  ;[0.05 0.25 0.4 0.6] 攻撃：モーション再生後、まだ範囲内ならダメージ。間隔をあけて繰り返す
  (`/Engine/EditorBlueprintResources/StandardMacros.IsValid` (`self.AttackTarget`)
    (:`Is Valid`
      (`AnimInstance.PlaySlotAnimationAsDynamicMontage` (`SkeletalMeshComponent.GetAnimInstance` (`self.Mesh`)) "/Game/Characters/Mannequins/Anims/Unarmed/Attack/MM_Attack_01.MM_Attack_01" "DefaultSlot" 0.1 0.2 1.2 1 -1.0 0.0)
      (`GameplayStatics.PlaySoundAtLocation` "/Game/ChronoVault/Audio/SE/SE_Attack.SE_Attack" (`self.K2_GetActorLocation`) (struct) 1.0 1.0 0.0 null null null null)
      (`KismetSystemLibrary.Delay` 0.4)
      (`/Engine/EditorBlueprintResources/StandardMacros.IsValid` (`self.AttackTarget`)
        (:`Is Valid`
          (`GameplayStatics.ApplyDamage` (`self.AttackTarget`) (`self.AttackDamage`) null self))))))

(event `self.AttackSphere.OnComponentBeginOverlap`
  (params (OverlappedComponent :type "PrimitiveComponent Object Reference") (OtherActor :type "Actor Object Reference") (OtherComp :type "PrimitiveComponent Object Reference") (OtherBodyIndex :type Integer) (bFromSweep :type Boolean) (SweepResult :type "HitResult Structure (by ref)"))
  ;[0.1 0.35 0.15 0.6] 攻撃範囲に入ったら攻撃開始
  (if (`KismetSystemLibrary.DoesImplementInterface` OtherActor "/Game/ChronoVault/Player/BPI_Player.BPI_Player_C")
    (set `self.AttackTarget` OtherActor)
    (`self.TryAttack`)
    (`KismetSystemLibrary.K2_SetTimer` self "TryAttack" (`self.AttackInterval`) true)))

(event `self.AttackSphere.OnComponentEndOverlap`
  (params (OverlappedComponent :type "PrimitiveComponent Object Reference") (OtherActor :type "Actor Object Reference") (OtherComp :type "PrimitiveComponent Object Reference") (OtherBodyIndex :type Integer))
  ;[0.4 0.25 0.05 0.6] 攻撃範囲から出たら攻撃停止
  (if (== OtherActor (`self.AttackTarget`))
    (set `self.AttackTarget` null)
    (`KismetSystemLibrary.K2_ClearTimer` self "TryAttack")))

(event `self.ReceiveBeginPlay`
  ;[0.3 0.1 0.35 0.6] 初期化：巡回速度で開始
  (set `CharacterMovementComponent.MaxWalkSpeed` (`self.PatrolSpeed`) (`self.CharacterMovement`))
  (`self.SetAlertState` 0))

(fn `GetNextPatrolPoint`
  (returns (NextPoint :type "Actor Object Reference"))
  ;[0.05 0.25 0.4 0.6] 次の巡回ポイントを返し、番号を1つ進める（末尾なら先頭へ）
  (if (> (`KismetArrayLibrary.Array_Length` (`self.PatrolPoints`)) 0)
    (set `self.PatrolPointIndex` (mod (+ (`self.PatrolPointIndex`) 1) (`KismetArrayLibrary.Array_Length` (`self.PatrolPoints`))))
    (return (`|GetArrayItem` (`self.PatrolPoints`) (`self.PatrolPointIndex`)))
    (else
      (return null))))

(fn `SetAlertState`
  (params (AlertState :type Integer))
  ;[0.05 0.25 0.4 0.6] 頭上マークの切替（0:なし 1:！ 2:？）
  (bind _asuw_alert (cast `/Game/ChronoVault/UI/UW_Alert` (`WidgetComponent.GetUserWidgetObject` (`self.AlertWidget`))))
  (`/Game/ChronoVault/UI/UW_Alert.SetAlertState` _asuw_alert AlertState))

(fn `SetDiscovered`
  (params (bNewDiscovered :type Boolean))
  (bind _returnvalue (`self.K2_GetActorLocation`))
  ;[0.05 0.25 0.4 0.6] 発見/見失いで速度・ライト色・マーク・SEを切替
  (set `self.bDiscovered` bNewDiscovered)
  (if bNewDiscovered
    (set `CharacterMovementComponent.MaxWalkSpeed` (`self.ChaseSpeed`) (`self.CharacterMovement`))
    (`self.SetAlertState` 1)
    (`LightComponent.SetLightColor` (`self.EyeLight`) (struct :`R` 1.0 :`G` 0.05 :`B` 0.02 :`A` 1.0) true)
    (`GameplayStatics.PlaySoundAtLocation` "/Game/ChronoVault/Audio/SE/SE_Alert.SE_Alert" _returnvalue (struct) 1.0 1.0 0.0 null null null null)
    (else
      (set `CharacterMovementComponent.MaxWalkSpeed` (`self.PatrolSpeed`) (`self.CharacterMovement`))
      (`self.SetAlertState` 2)
      (`LightComponent.SetLightColor` (`self.EyeLight`) (struct :`R` 1.0 :`G` 0.55 :`B` 0.08 :`A` 1.0) true)
      (`GameplayStatics.PlaySoundAtLocation` "/Game/ChronoVault/Audio/SE/SE_Lost.SE_Lost" _returnvalue (struct) 1.0 1.0 0.0 null null null null))))

(fn `UserConstructionScript`)