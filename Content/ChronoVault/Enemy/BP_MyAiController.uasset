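; AI Controller for the BP_MyCharacter enemy that switches it between discovered and searching states as it senses players.
; It starts BB_MyCharacter and BT_MyCharacter on BeginPlay and caches the possessed enemy.
; AIPerception updates filter actors by BPI_Player, then FindPlayer sets the chase target or LostPlayer stores the last seen location for searching.
; Both update Blackboard keys, set the enemy's discovered flag and notify the player of detection changes.
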(event `self.ReceiveBeginPlay`
  ;[0.05 0.25 0.4 0.6] Blackboard と Behavior Tree を起動
  (`self.UseBlackboard` "/Game/ChronoVault/Enemy/BB_MyCharacter.BB_MyCharacter")
  (`self.RunBehaviorTree` "/Game/ChronoVault/Enemy/BT_MyCharacter.BT_MyCharacter"))

(event `self.ReceivePossess`
  (params (PossessedPawn :type "Pawn Object Reference"))
  ;[0.1 0.35 0.15 0.6] 操作対象の敵を記憶
  (bind _asbp_my_character (cast `/Game/ChronoVault/Enemy/BP_MyCharacter` PossessedPawn))
  (set `self.EnemyCharacter` _asbp_my_character))

(event `self.AIPerception.OnPerceptionUpdated`
  (params (UpdatedActors :type "Array of Actor Object Reference (by ref)"))
  ;[0.4 0.25 0.05 0.6] 視覚の更新：プレイヤーを発見 / 見失いで Blackboard を更新
  (for _array_element UpdatedActors
    (if (`KismetSystemLibrary.DoesImplementInterface` _array_element "/Game/ChronoVault/Player/BPI_Player.BPI_Player_C")
      (bind _info (`AIPerceptionComponent.GetActorsPerception` (`self.AIPerception`) _array_element))
      (bind (_age _expirationage _strength _stimuluslocation _receiverlocation _tag _bsuccessfullysensed) (break `AIStimulus` (`|GetArrayItem` (`.LastSensedStimuli` (break `ActorPerceptionBlueprintInfo` _info)))))
      (if _bsuccessfullysensed
        (`self.FindPlayer` _array_element)
        (else
          (`self.LostPlayer` _array_element _stimuluslocation))))))

(fn `FindPlayer`
  (params (SensedActor :type "Actor Object Reference"))
  ;[0.05 0.25 0.4 0.6] 発見：追跡対象を設定し、追跡状態へ
  (`BlackboardComponent.SetValueAsObject` (`self.Blackboard`) (`self.Key_TargetActor`) SensedActor)
  (`BlackboardComponent.SetValueAsBool` (`self.Blackboard`) (`self.Key_bDiscovered`) true)
  (`BlackboardComponent.SetValueAsBool` (`self.Blackboard`) (`self.Key_bSearching`) false)
  (`/Game/ChronoVault/Enemy/BP_MyCharacter.SetDiscovered` (`self.EnemyCharacter`) true)
  (message `/Game/ChronoVault/Player/BPI_Player.PlayerSetDetected` SensedActor true (`self.EnemyCharacter`)))

(fn `LostPlayer`
  (params (LostActor :type "Actor Object Reference") (LastLocation :type "Vector Structure"))
  ;[0.05 0.25 0.4 0.6] 見失い：最後に見た場所を調べてから巡回へ復帰
  (`BlackboardComponent.SetValueAsVector` (`self.Blackboard`) (`self.Key_LastKnownLocation`) LastLocation)
  (`BlackboardComponent.SetValueAsBool` (`self.Blackboard`) (`self.Key_bSearching`) true)
  (`BlackboardComponent.SetValueAsBool` (`self.Blackboard`) (`self.Key_bDiscovered`) false)
  (`BlackboardComponent.ClearValue` (`self.Blackboard`) (`self.Key_TargetActor`))
  (`/Game/ChronoVault/Enemy/BP_MyCharacter.SetDiscovered` (`self.EnemyCharacter`) false)
  (message `/Game/ChronoVault/Player/BPI_Player.PlayerSetDetected` LostActor false (`self.EnemyCharacter`)))

(fn `UserConstructionScript`)