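; Game instance that holds the player's progress across levels and persists it to a single save slot.
; On Init it loads event and key flags, save transform, item names, play time and death count from BP_MySaveGame, resetting most of them if loading fails.
; Export writes the state back, Delete clears slot and state, and Retry reloads while preserving play time and death count.
; Setter and getter functions expose the event and key maps by name.
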(event `self.ReceiveInit`
  ;[0.05 0.25 0.4 0.6] 起動時：セーブデータを読み込む
  (`self.ImportSaveData`))

(fn `DeleteSaveData`
  ;[0.05 0.25 0.4 0.6] セーブスロットを削除し初期化する（開発用リセット / はじめから）
  (`GameplayStatics.DeleteGameInSlot` (`self.SlotName`))
  (`self.ResetData`))

(fn `ExportSaveData`
  ;[0.05 0.25 0.4 0.6] SaveGameオブジェクトへ書き出し、スロットに保存する
  (bind _returnvalue (`GameplayStatics.CreateSaveGameObject` "/Game/ChronoVault/Save/BP_MySaveGame.BP_MySaveGame_C"))
  (set `self.SaveGameObject` _returnvalue)
  (set `/Game/ChronoVault/Save/BP_MySaveGame.EventStatus` (`self.EventStatus`) (`self.SaveGameObject`))
  (set `/Game/ChronoVault/Save/BP_MySaveGame.KeyStatus` (`self.KeyStatus`) (`self.SaveGameObject`))
  (set `/Game/ChronoVault/Save/BP_MySaveGame.PlayerSaveTransform` (`self.PlayerSaveTransform`) (`self.SaveGameObject`))
  (set `/Game/ChronoVault/Save/BP_MySaveGame.PlayerItemNameList` (`self.PlayerItemNameList`) (`self.SaveGameObject`))
  (set `/Game/ChronoVault/Save/BP_MySaveGame.PlayTime` (`self.PlayTime`) (`self.SaveGameObject`))
  (set `/Game/ChronoVault/Save/BP_MySaveGame.DeathCount` (`self.DeathCount`) (`self.SaveGameObject`))
  (`GameplayStatics.SaveGameToSlot` (`self.SaveGameObject`) (`self.SlotName`))
  (set `self.bHasSaveData` true))

(fn `GetEventStatus`
  (params (EventName :type Name))
  (returns (bFinished :type Boolean))
  (return (`BlueprintMapLibrary.Map_Find` (`self.EventStatus`) EventName)))

(fn `GetKeyStatus`
  (params (KeyName :type Name))
  (returns (bTaken :type Boolean))
  (return (`BlueprintMapLibrary.Map_Find` (`self.KeyStatus`) KeyName)))

(fn `ImportSaveData`
  (returns (bSuccess :type Boolean))
  ;[0.05 0.25 0.4 0.6] スロットから読み込む。無ければ初期化する
  (bind _returnvalue (`GameplayStatics.DoesSaveGameExist` (`self.SlotName`)))
  (if _returnvalue
    (bind _returnvalue_2 (`GameplayStatics.LoadGameFromSlot` (`self.SlotName`)))
    (bind _asbp_my_save_game (cast `/Game/ChronoVault/Save/BP_MySaveGame` _returnvalue_2)
      (:`then`
        (set `self.SaveGameObject` _asbp_my_save_game)
        (set `self.EventStatus` (`/Game/ChronoVault/Save/BP_MySaveGame.EventStatus` (`self.SaveGameObject`)))
        (set `self.KeyStatus` (`/Game/ChronoVault/Save/BP_MySaveGame.KeyStatus` (`self.SaveGameObject`)))
        (set `self.PlayerSaveTransform` (`/Game/ChronoVault/Save/BP_MySaveGame.PlayerSaveTransform` (`self.SaveGameObject`)))
        (set `self.PlayerItemNameList` (`/Game/ChronoVault/Save/BP_MySaveGame.PlayerItemNameList` (`self.SaveGameObject`)))
        (set `self.PlayTime` (`/Game/ChronoVault/Save/BP_MySaveGame.PlayTime` (`self.SaveGameObject`)))
        (set `self.DeathCount` (`/Game/ChronoVault/Save/BP_MySaveGame.DeathCount` (`self.SaveGameObject`)))
        (set `self.bHasSaveData` true)
        (return true))
      (:`CastFailed`
        _)))
  (`self.ResetData`)
  (return false))

(fn `ResetData`
  ;[0.05 0.25 0.4 0.6] 進行データを初期状態に戻す
  (`BlueprintMapLibrary.Map_Clear` (`self.EventStatus`))
  (`BlueprintMapLibrary.Map_Clear` (`self.KeyStatus`))
  (`KismetArrayLibrary.Array_Clear` (`self.PlayerItemNameList`))
  (set `self.PlayTime` 0.0)
  (set `self.DeathCount` 0)
  (set `self.bHasSaveData` false))

(fn `RetryFromSave`
  ;[0.05 0.25 0.4 0.6] 最後のセーブ時点へ戻す。プレイ時間と死亡回数だけは引き継ぐ
  (set `self.PreviousPlayTime` (`self.PlayTime`))
  (set `self.PreviousDeathCount` (`self.DeathCount`))
  (`self.ImportSaveData`)
  (set `self.PlayTime` (`self.PreviousPlayTime`))
  (set `self.DeathCount` (`self.PreviousDeathCount`)))

(fn `SetEventStatus`
  (params (EventName :type Name) (bFinished :type Boolean))
  (`BlueprintMapLibrary.Map_Add` (`self.EventStatus`) EventName bFinished))

(fn `SetKeyStatus`
  (params (KeyName :type Name) (bTaken :type Boolean))
  (`BlueprintMapLibrary.Map_Add` (`self.KeyStatus`) KeyName bTaken))