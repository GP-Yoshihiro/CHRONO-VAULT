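; BP_MyGameMode is the game mode that runs game over, level clear and music switching for the player's run.
; On begin play it starts exploration music, prepares chase music, and binds to BP_Player's death and detection dispatchers to show game over or crossfade tracks.
; Game over waits a delay before its widget, while clear pauses and shows its own.
; A GameEnded flag guards both endings and stops play time accumulating in the GameInstance, which also counts deaths.
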(event `GameOver`
  (bind _asbp_my_game_instance (cast `/Game/ChronoVault/Core/BP_MyGameInstance` (`GameplayStatics.GetGameInstance`) :!pure true))
  ;[0.05 0.25 0.4 0.6] 死亡通知 → 演出を待ってゲームオーバー画面を表示
  (if (not (`self.bGameEnded`))
    (set `self.bGameEnded` true)
    (set `/Game/ChronoVault/Core/BP_MyGameInstance.DeathCount` (+ (`/Game/ChronoVault/Core/BP_MyGameInstance.DeathCount` _asbp_my_game_instance) 1) _asbp_my_game_instance)
    (`KismetSystemLibrary.Delay` (`self.GameOverDelay`))
    (bind _returnvalue (`|CreateWidget` "/Game/ChronoVault/UI/WBP_GameOver.WBP_GameOver_C" (`GameplayStatics.GetPlayerController` 0)))
    (`UserWidget.AddToViewport` _returnvalue 20)))

(event `GameClear`
  ;[0.1 0.35 0.15 0.6] ゴール到達 → クリア画面を表示
  (if (not (`self.bGameEnded`))
    (set `self.bGameEnded` true)
    (`GameplayStatics.SetGamePaused` true)
    (bind _returnvalue (`|CreateWidget` "/Game/ChronoVault/UI/WBP_Clear.WBP_Clear_C" (`GameplayStatics.GetPlayerController` 0)))
    (`UserWidget.AddToViewport` _returnvalue 20)))

(event `ChangeChaseBgm`
  (params (bDetected :type Boolean))
  ;[0.4 0.25 0.05 0.6] 発見状態に応じて探索BGMと追跡BGMを切替
  (if (and (`KismetSystemLibrary.IsValid` (`self.BgmExplore`)) (`KismetSystemLibrary.IsValid` (`self.BgmChase`)))
    (if bDetected
      (`AudioComponent.FadeOut` (`self.BgmExplore`) 0.6 0.0 "Linear")
      (`AudioComponent.FadeIn` (`self.BgmChase`) 0.3 0.5 0.0 "Linear")
      (else
        (`AudioComponent.FadeOut` (`self.BgmChase`) 1.5 0.0 "Linear")
        (`AudioComponent.FadeIn` (`self.BgmExplore`) 1.5 0.5 0.0 "Linear")))))

(event `self.ReceiveBeginPlay`
  ;[0.3 0.1 0.35 0.6] 開始：BGM再生、プレイヤーのディスパッチャーにバインド
  (bind _returnvalue (`GameplayStatics.SpawnSound2D` "/Game/ChronoVault/Audio/BGM/BGM_Explore.BGM_Explore" 0.5 1.0 0.0 null false false))
  (set `self.BgmExplore` _returnvalue)
  (bind _returnvalue_2 (`GameplayStatics.CreateSound2D` "/Game/ChronoVault/Audio/BGM/BGM_Chase.BGM_Chase" 0.5 1.0 0.0 null false false))
  (set `self.BgmChase` _returnvalue_2)
  (`KismetSystemLibrary.DelayUntilNextTick`)
  (bind _asbp_player (cast `/Game/ChronoVault/Player/BP_Player` (`GameplayStatics.GetPlayerPawn` 0)))
  (add `/Game/ChronoVault/Player/BP_Player.OnPlayerDead` _asbp_player (delegate `GameOver`))
  (add `/Game/ChronoVault/Player/BP_Player.OnDetectedChanged` _asbp_player (delegate `ChangeChaseBgm`)))

(event `self.ReceiveTick`
  (params (DeltaSeconds :type "Float (single-precision)"))
  (bind _asbp_my_game_instance (cast `/Game/ChronoVault/Core/BP_MyGameInstance` (`GameplayStatics.GetGameInstance`) :!pure true))
  ;[0.4 0.08 0.1 0.6] プレイ時間の加算
  (if (not (`self.bGameEnded`))
    (set `/Game/ChronoVault/Core/BP_MyGameInstance.PlayTime` (+ (`/Game/ChronoVault/Core/BP_MyGameInstance.PlayTime` _asbp_my_game_instance) DeltaSeconds) _asbp_my_game_instance)))

(fn `UserConstructionScript`)