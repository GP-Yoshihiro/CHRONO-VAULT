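; BP_Player is the player character, with Enhanced Input movement, dash, interaction, pause and a debug save reset.
; An overlap sphere picks BPI_Interact targets and shows their prompts.
; Damage triggers a screen flash, brief invincibility or death.
; BPI_Player handles items, messages, detecting-enemy tracking and saving/loading through BP_MyGameInstance, while event dispatchers announce HP, item, detection and death changes.
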(event `self.ReceiveBeginPlay`
  (bind _returnvalue (`GameplayStatics.GetPlayerController` 0))
  ;[0.05 0.25 0.4 0.6] 初期化：入力コンテキスト登録 → UI生成 → 次Tickでセーブデータ反映
  (`EnhancedInputSubsystemInterface.AddMappingContext` (pcsubsystem `EnhancedInputLocalPlayerSubsystem` _returnvalue) "/Game/ChronoVault/Input/IMC_MyDefault.IMC_MyDefault" 0 (struct))
  (`/Game/ChronoVault/Core/BP_MyPlayerController.SetMenuMode` (cast `/Game/ChronoVault/Core/BP_MyPlayerController` (`GameplayStatics.GetPlayerController` 0) :!pure true) false)
  (bind _returnvalue_2 (`|CreateWidget` "/Game/ChronoVault/UI/UW_GameUI.UW_GameUI_C" _returnvalue))
  (set `self.GameUI` _returnvalue_2)
  (`UserWidget.AddToViewport` (`self.GameUI`) 0)
  (bind _returnvalue_3 (`|CreateWidget` "/Game/ChronoVault/UI/UW_ScreenEffect.UW_ScreenEffect_C" _returnvalue))
  (set `self.ScreenEffectUI` _returnvalue_3)
  (`UserWidget.AddToViewport` (`self.ScreenEffectUI`) 5)
  (set `self.CurrentHp` (`self.MaxHp`))
  (`KismetSystemLibrary.DelayUntilNextTick`)
  (message `/Game/ChronoVault/Player/BPI_Player.PlayerLoadData` self)
  (`self.OnCharacterHpChanged` (`self.CurrentHp`) (`self.MaxHp`)))

(event `EnhancedInput|/Game/ChronoVault/Input/IA_Move`
  (params (ActionValue :type "Vector2D Structure") (ElapsedSeconds :type "Float (double-precision)") (TriggeredSeconds :type "Float (double-precision)") (InputAction :type "InputAction Object Reference" :default "/Game/ChronoVault/Input/IA_Move.IA_Move"))
  (bind (_x _y) (`KismetMathLibrary.BreakVector2D` ActionValue))
  (bind _returnvalue (`KismetMathLibrary.MakeRotator` 0.0 0.0 (.yaw (`self.GetControlRotation`))))
  ;[0.1 0.35 0.15 0.6] 移動：カメラの向きを基準に前後左右へ移動（IMC_MyDefault）
  (:`Triggered`
    (`self.AddMovementInput` (`KismetMathLibrary.GetForwardVector` _returnvalue) _y)
    (`self.AddMovementInput` (`KismetMathLibrary.GetRightVector` _returnvalue) _x)))

(event `EnhancedInput|/Game/ChronoVault/Input/IA_Look`
  (params (ActionValue :type "Vector2D Structure") (ElapsedSeconds :type "Float (double-precision)") (TriggeredSeconds :type "Float (double-precision)") (InputAction :type "InputAction Object Reference" :default "/Game/ChronoVault/Input/IA_Look.IA_Look"))
  (bind (_x _y) (`KismetMathLibrary.BreakVector2D` ActionValue))
  ;[0.4 0.25 0.05 0.6] 視点操作
  (:`Triggered`
    (`self.AddControllerYawInput` _x)
    (`self.AddControllerPitchInput` _y)))

(event `EnhancedInput|/Game/ChronoVault/Input/IA_Jump`
  (params (ActionValue :type Boolean) (ElapsedSeconds :type "Float (double-precision)") (TriggeredSeconds :type "Float (double-precision)") (InputAction :type "InputAction Object Reference" :default "/Game/ChronoVault/Input/IA_Jump.IA_Jump"))
  ;[0.3 0.1 0.35 0.6] ジャンプ
  (:`Started`
    (`self.Jump`))
  (:`Completed`
    (`self.StopJumping`)))

(event `EnhancedInput|/Game/ChronoVault/Input/IA_Dash`
  (params (ActionValue :type Boolean) (ElapsedSeconds :type "Float (double-precision)") (TriggeredSeconds :type "Float (double-precision)") (InputAction :type "InputAction Object Reference" :default "/Game/ChronoVault/Input/IA_Dash.IA_Dash"))
  ;[0.4 0.08 0.1 0.6] ダッシュ：Shiftを押している間だけ移動速度を上げる
  (:`Started`
    (set `CharacterMovementComponent.MaxWalkSpeed` (`self.DashSpeed`) (`self.CharacterMovement`)))
  (:`Completed`
    (set `CharacterMovementComponent.MaxWalkSpeed` (`self.WalkSpeed`) (`self.CharacterMovement`))))

(event `EnhancedInput|/Game/ChronoVault/Input/IA_Interact`
  (params (ActionValue :type Boolean) (ElapsedSeconds :type "Float (double-precision)") (TriggeredSeconds :type "Float (double-precision)") (InputAction :type "InputAction Object Reference" :default "/Game/ChronoVault/Input/IA_Interact.IA_Interact"))
  ;[0.05 0.25 0.4 0.6] 操作：範囲内のレバー等を BPI_Interact 経由で操作（Castなし）
  (:`Started`
    (`/Engine/EditorBlueprintResources/StandardMacros.IsValid` (`self.InteractTarget`)
      (:`Is Valid`
        (message `/Game/ChronoVault/Gimmick/BPI_Interact.Interact` (`self.InteractTarget`) self)
        (`/Game/ChronoVault/UI/UW_GameUI.SetInteractText` (`self.GameUI`) "" false)))))

(event `EnhancedInput|/Game/ChronoVault/Input/IA_Pause`
  (params (ActionValue :type Boolean) (ElapsedSeconds :type "Float (double-precision)") (TriggeredSeconds :type "Float (double-precision)") (InputAction :type "InputAction Object Reference" :default "/Game/ChronoVault/Input/IA_Pause.IA_Pause"))
  ;[0.1 0.35 0.15 0.6] ポーズ画面を開く
  (:`Started`
    (if (not (`self.bIsDead`))
      (bind _returnvalue (`|CreateWidget` "/Game/ChronoVault/UI/WBP_Pause.WBP_Pause_C" (`GameplayStatics.GetPlayerController` 0)))
      (`UserWidget.AddToViewport` _returnvalue 10))))

(event `EnhancedInput|/Game/ChronoVault/Input/IA_DebugReset`
  (params (ActionValue :type Boolean) (ElapsedSeconds :type "Float (double-precision)") (TriggeredSeconds :type "Float (double-precision)") (InputAction :type "InputAction Object Reference" :default "/Game/ChronoVault/Input/IA_DebugReset.IA_DebugReset"))
  ;[0.4 0.25 0.05 0.6] 開発用：R長押しでセーブデータを削除し最初から
  (:`Triggered`
    (`/Game/ChronoVault/Core/BP_MyGameInstance.DeleteSaveData` (cast `/Game/ChronoVault/Core/BP_MyGameInstance` (`GameplayStatics.GetGameInstance`) :!pure true))
    (`GameplayStatics.OpenLevel` "/Game/ChronoVault/Levels/L_ChronoVault")))

(event `self.InteractSphere.OnComponentBeginOverlap`
  (params (OverlappedComponent :type "PrimitiveComponent Object Reference") (OtherActor :type "Actor Object Reference") (OtherComp :type "PrimitiveComponent Object Reference") (OtherBodyIndex :type Integer) (bFromSweep :type Boolean) (SweepResult :type "HitResult Structure (by ref)"))
  ;[0.3 0.1 0.35 0.6] 操作可能な物が範囲に入ったらプロンプト表示
  (if (`KismetSystemLibrary.DoesImplementInterface` OtherActor "/Game/ChronoVault/Gimmick/BPI_Interact.BPI_Interact_C")
    (set `self.InteractTarget` OtherActor)
    (bind _interacttext (message `/Game/ChronoVault/Gimmick/BPI_Interact.GetInteractText` (`self.InteractTarget`)))
    (`/Game/ChronoVault/UI/UW_GameUI.SetInteractText` (`self.GameUI`) _interacttext (not (`KismetTextLibrary.TextIsEmpty` _interacttext)))))

(event `self.InteractSphere.OnComponentEndOverlap`
  (params (OverlappedComponent :type "PrimitiveComponent Object Reference") (OtherActor :type "Actor Object Reference") (OtherComp :type "PrimitiveComponent Object Reference") (OtherBodyIndex :type Integer))
  ;[0.4 0.08 0.1 0.6] 範囲から出たらプロンプト非表示
  (if (== OtherActor (`self.InteractTarget`))
    (set `self.InteractTarget` null)
    (`/Game/ChronoVault/UI/UW_GameUI.SetInteractText` (`self.GameUI`) "" false)))

(event `Die`
  ;[0.05 0.25 0.4 0.6] 死亡：操作を止めて倒れ演出を再生し、OnPlayerDead を通知
  (set `self.bIsDead` true)
  (`self.DisableInput` (`GameplayStatics.GetPlayerController` 0))
  (`CharacterMovementComponent.DisableMovement` (`self.CharacterMovement`))
  (`SkeletalMeshComponent.PlayAnimation` (`self.Mesh`) "/Game/Characters/Mannequins/Anims/Death/MM_Death_Front_01.MM_Death_Front_01" false)
  (`self.OnPlayerDead`))

(event `self.ReceiveAnyDamage`
  (params (Damage :type "Float (single-precision)") (DamageType :type "DamageType Object Reference") (InstigatedBy :type "Controller Object Reference") (DamageCauser :type "Actor Object Reference"))
  ;[0.1 0.35 0.15 0.6] ダメージ：HPを減らし、UIへ通知。HPが0なら死亡、残っていれば短時間無敵
  (if (not (or (`self.bIsDead`) (`self.bInvincible`)))
    (set `self.CurrentHp` (`KismetMathLibrary.FClamp` (- (`self.CurrentHp`) Damage) 0.0 (`self.MaxHp`)))
    (`self.OnCharacterHpChanged` (`self.CurrentHp`) (`self.MaxHp`))
    (message `/Game/ChronoVault/Player/BPI_Player.PlayerPlayScreenEffect` self (struct :`R` 1.0 :`A` 1.0))
    (`GameplayStatics.PlaySound2D` "/Game/ChronoVault/Audio/SE/SE_Damage.SE_Damage" 1.0 1.0 0.0 null null)
    (if (<= (`self.CurrentHp`) 0.0)
      (`self.Die`)
      (else
        (set `self.bInvincible` true)
        (`KismetSystemLibrary.Delay` (`self.InvincibleTime`))
        (set `self.bInvincible` false)))))

(event `/Game/ChronoVault/Player/BPI_Player.PlayerPlayScreenEffect`
  (params (EffectColor :type "LinearColor Structure"))
  ;[0.4 0.25 0.05 0.6] BPI_Player：画面フラッシュ再生
  (`/Game/ChronoVault/UI/UW_ScreenEffect.PlayFlash` (`self.ScreenEffectUI`) EffectColor))

(event `/Game/ChronoVault/Player/BPI_Player.PlayerSaveData`
  (params (SaveTransform :type "Transform Structure"))
  (bind _asbp_my_game_instance (cast `/Game/ChronoVault/Core/BP_MyGameInstance` (`GameplayStatics.GetGameInstance`) :!pure true))
  ;[0.3 0.1 0.35 0.6] BPI_Player：現在の進行を GameInstance に渡し SaveGame へ書き出す
  (set `/Game/ChronoVault/Core/BP_MyGameInstance.PlayerSaveTransform` SaveTransform _asbp_my_game_instance)
  (set `/Game/ChronoVault/Core/BP_MyGameInstance.PlayerItemNameList` (`self.ItemNameList`) _asbp_my_game_instance)
  (`/Game/ChronoVault/Core/BP_MyGameInstance.ExportSaveData` _asbp_my_game_instance)
  (message `/Game/ChronoVault/Player/BPI_Player.PlayerShowMessage` self "セーブしました" 2.0))

(event `/Game/ChronoVault/Player/BPI_Player.PlayerLoadData`
  (bind _asbp_my_game_instance (cast `/Game/ChronoVault/Core/BP_MyGameInstance` (`GameplayStatics.GetGameInstance`) :!pure true))
  (bind _rotation (.rotation (`/Game/ChronoVault/Core/BP_MyGameInstance.PlayerSaveTransform` _asbp_my_game_instance)))
  ;[0.4 0.08 0.1 0.6] BPI_Player：セーブがあれば所持品 → 位置と向きの順に復元
  (if (`/Game/ChronoVault/Core/BP_MyGameInstance.bHasSaveData` _asbp_my_game_instance)
    (set `self.ItemNameList` (`/Game/ChronoVault/Core/BP_MyGameInstance.PlayerItemNameList` _asbp_my_game_instance))
    (`self.K2_SetActorLocationAndRotation` (.location (`/Game/ChronoVault/Core/BP_MyGameInstance.PlayerSaveTransform` _asbp_my_game_instance)) _rotation false true)
    (`Controller.SetControlRotation` (`self.GetController`) _rotation))
  (`self.OnItemChanged`))

(event `/Game/ChronoVault/Player/BPI_Player.PlayerAddItem`
  (params (ItemName :type Name))
  ;[0.05 0.25 0.4 0.6] BPI_Player：アイテム取得
  (`KismetArrayLibrary.Array_AddUnique` (`self.ItemNameList`) ItemName)
  (`self.OnItemChanged`))

(event `/Game/ChronoVault/Player/BPI_Player.PlayerShowMessage`
  (params (Message :type Text) (Duration :type "Float (double-precision)"))
  ;[0.1 0.35 0.15 0.6] BPI_Player：メッセージ表示
  (`/Game/ChronoVault/UI/UW_GameUI.ShowMessage` (`self.GameUI`) Message Duration))

(event `/Game/ChronoVault/Player/BPI_Player.PlayerSetDetected`
  (params (bDetected :type Boolean) (Enemy :type "Actor Object Reference"))
  ;[0.4 0.25 0.05 0.6] BPI_Player：発見している敵を管理し、警告UIとBGMへ通知
  (if bDetected
    (`KismetArrayLibrary.Array_AddUnique` (`self.DetectedEnemies`) Enemy)
    (else
      (`KismetArrayLibrary.Array_RemoveItem` (`self.DetectedEnemies`) Enemy)))
  (`self.OnDetectedChanged` (> (`KismetArrayLibrary.Array_Length` (`self.DetectedEnemies`)) 0)))

(fn `PlayerHasItem`
  (params (ItemName :type Name))
  (returns (bHasItem :type Boolean))
  ;[0.05 0.25 0.4 0.6] 指定アイテムを所持しているか
  (return (`KismetArrayLibrary.Array_Contains` (`self.ItemNameList`) ItemName)))

(fn `UserConstructionScript`)