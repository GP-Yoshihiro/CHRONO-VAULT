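; BP_Door is a gimmick sliding double door that opens either when touched by a player holding all required keys or when activated with all required events complete.
; Touch mode checks items through BPI_Player and shows amber lamps; activation checks event status in BP_MyGameInstance.
; Opening marks it finished, turns lamps green and drives both panels through a timeline.
; Failed touches show a locked message, and restore snaps it open.
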(event `OpenDoor`
  ;[0.05 0.25 0.4 0.6] 扉を開く：作動済みを記録し、タイムラインでスライド
  (`self.MarkFinished`)
  (`self.SetLampGreen`)
  (`GameplayStatics.PlaySoundAtLocation` "/Game/ChronoVault/Audio/SE/SE_Door.SE_Door" (`self.K2_GetActorLocation`) (struct) 1.0 1.0 0.0 null null null null)
  (bind (_direction _openrate) (`Timeline|DoorTimeline`)
    (:`Update`
      (`self.SetOpenRate` _openrate))))

(event `self.OnActivate`
  (params (GimmickInstigator :type "Actor Object Reference"))
  ;[0.1 0.35 0.15 0.6] スイッチ/レバーからの作動：必要イベントが揃えば開く
  (bind _ballevents (`self.CheckEvents`))
  (if _ballevents
    (`self.OpenDoor`)))

(event `self.OnRestore`
  ;[0.4 0.25 0.05 0.6] 復元：最初から開いた状態にする
  (`self.SetOpenRate` 1.0)
  (`self.SetLampGreen`))

(event `self.Trigger.OnComponentBeginOverlap`
  (params (OverlappedComponent :type "PrimitiveComponent Object Reference") (OtherActor :type "Actor Object Reference") (OtherComp :type "PrimitiveComponent Object Reference") (OtherBodyIndex :type Integer) (bFromSweep :type Boolean) (SweepResult :type "HitResult Structure (by ref)"))
  ;[0.3 0.1 0.35 0.6] プレイヤー接触：鍵判定で開く。足りなければメッセージ
  (if (and (`KismetSystemLibrary.DoesImplementInterface` OtherActor "/Game/ChronoVault/Player/BPI_Player.BPI_Player_C") (not (`self.bFinished`)))
    (if (`self.bOpenByTouch`)
      (bind _ballkeys (`self.CheckKeys` OtherActor))
      (if _ballkeys
        (`self.OpenDoor`)
        (else
          (message `/Game/ChronoVault/Player/BPI_Player.PlayerShowMessage` OtherActor (`self.LockedMessage`) 2.5 :!label _label)
          (`GameplayStatics.PlaySound2D` "/Game/ChronoVault/Audio/SE/SE_Locked.SE_Locked" 1.0 1.0 0.0 null null)))
      (else
        (goto _label)))))

(fn `CheckEvents`
  (returns (bAllEvents :type Boolean))
  ;[0.05 0.25 0.4 0.6] 必要なイベントがすべて完了しているか
  (for _array_element (`self.RequiredEvents`)
    (if (not (`/Game/ChronoVault/Core/BP_MyGameInstance.GetEventStatus` (cast `/Game/ChronoVault/Core/BP_MyGameInstance` (`GameplayStatics.GetGameInstance`) :!pure true) _array_element))
      (return false)))
  (return true))

(fn `CheckKeys`
  (params (PlayerActor :type "Actor Object Reference"))
  (returns (bAllKeys :type Boolean))
  ;[0.05 0.25 0.4 0.6] 必要な鍵をすべて持っているか（BPI_Player経由）
  (for _array_element (`self.RequiredKeys`)
    (bind _bhasitem (message `/Game/ChronoVault/Player/BPI_Player.PlayerHasItem` PlayerActor _array_element))
    (if (not _bhasitem)
      (return false)))
  (return true))

(fn `SetLampGreen`
  (`PrimitiveComponent.SetMaterial` (`self.LampFront`) 0 "/Game/ChronoVault/Materials/Instances/MI_LampGreen.MI_LampGreen")
  (`PrimitiveComponent.SetMaterial` (`self.LampBack`) 0 "/Game/ChronoVault/Materials/Instances/MI_LampGreen.MI_LampGreen"))

(fn `SetOpenRate`
  (params (Rate :type "Float (double-precision)"))
  (bind _returnvalue (+ (* Rate (`self.SlideDistance`)) 75.0))
  ;[0.05 0.25 0.4 0.6] 開き具合(0〜1)に応じて左右パネルをスライド
  (`SceneComponent.K2_SetRelativeLocation` (`self.PanelR`) (`KismetMathLibrary.MakeVector` 0.0 _returnvalue 165.0) false false)
  (`SceneComponent.K2_SetRelativeLocation` (`self.PanelL`) (`KismetMathLibrary.MakeVector` 0.0 (* _returnvalue -1.0) 165.0) false false))

(fn `UserConstructionScript`
  ;[0.05 0.25 0.4 0.6] 鍵で開く扉はランプを橙色にして区別する
  (if (`self.bOpenByTouch`)
    (`PrimitiveComponent.SetMaterial` (`self.LampFront`) 0 "/Game/ChronoVault/Materials/Instances/MI_LampAmber.MI_LampAmber")
    (`PrimitiveComponent.SetMaterial` (`self.LampBack`) 0 "/Game/ChronoVault/Materials/Instances/MI_LampAmber.MI_LampAmber")))