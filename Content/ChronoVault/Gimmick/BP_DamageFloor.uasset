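; BP_DamageFloor is a trap floor that repeatedly damages a player standing on its trigger.
; Overlap by a BPI_Player actor stores it as the single target, shows a warning message, deals immediate damage and starts a looping damage timer, cleared when that target leaves.
; An optional blink timer toggles the trap's active state and mesh visibility, with damage applied only while active and immediately upon reactivation.
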(event `self.Trigger.OnComponentBeginOverlap`
  (params (OverlappedComponent :type "PrimitiveComponent Object Reference") (OtherActor :type "Actor Object Reference") (OtherComp :type "PrimitiveComponent Object Reference") (OtherBodyIndex :type Integer) (bFromSweep :type Boolean) (SweepResult :type "HitResult Structure (by ref)"))
  ;[0.05 0.25 0.4 0.6] 乗ったら一定間隔のダメージ開始
  (if (`KismetSystemLibrary.DoesImplementInterface` OtherActor "/Game/ChronoVault/Player/BPI_Player.BPI_Player_C")
    (set `self.TargetActor` OtherActor)
    (`KismetSystemLibrary.K2_SetTimer` self "ApplyTrapDamage" (`self.DamageInterval`) true)
    (message `/Game/ChronoVault/Player/BPI_Player.PlayerShowMessage` OtherActor "危険！ ダメージ床だ" 1.5)
    (`self.ApplyTrapDamage`)))

(event `ApplyTrapDamage`
  ;[0.1 0.35 0.15 0.6] ONのとき対象にダメージを与える
  (if (and (`self.bTrapActive`) (`KismetSystemLibrary.IsValid` (`self.TargetActor`)))
    (`GameplayStatics.ApplyDamage` (`self.TargetActor`) (`self.Damage`) null self)))

(event `self.Trigger.OnComponentEndOverlap`
  (params (OverlappedComponent :type "PrimitiveComponent Object Reference") (OtherActor :type "Actor Object Reference") (OtherComp :type "PrimitiveComponent Object Reference") (OtherBodyIndex :type Integer))
  ;[0.4 0.25 0.05 0.6] 離れたらダメージ停止
  (if (== OtherActor (`self.TargetActor`))
    (set `self.TargetActor` null)
    (`KismetSystemLibrary.K2_ClearTimer` self "ApplyTrapDamage")))

(event `ToggleTrap`
  ;[0.3 0.1 0.35 0.6] 点滅トラップ：ON/OFFを切替え、見た目も変える
  (set `self.bTrapActive` (not (`self.bTrapActive`)))
  (`SceneComponent.SetVisibility` (`self.TrapMesh`) (`self.bTrapActive`) false)
  (if (`self.bTrapActive`)
    (`self.ApplyTrapDamage`)))

(event `self.ReceiveBeginPlay`
  ;[0.4 0.08 0.1 0.6] 点滅設定なら切替タイマー開始
  (if (`self.bBlink`)
    (`KismetSystemLibrary.K2_SetTimer` self "ToggleTrap" (`self.BlinkTime`) true)))

(fn `UserConstructionScript`)