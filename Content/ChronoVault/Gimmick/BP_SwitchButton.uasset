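; BP_SwitchButton is a gimmick switch that a player presses by stepping on it, activating its linked target gimmicks.
; A trigger overlap by a BPI_Player actor sends the activate message.
; OnActivate marks it finished, turns the lamp green, plays a sound, activates targets, shows the player a message and sinks the button through a timeline driving SetPressed.
; OnRestore reapplies the pressed position and green material instantly.
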(event `self.OnActivate`
  (params (GimmickInstigator :type "Actor Object Reference"))
  ;[0.05 0.25 0.4 0.6] 作動：ボタンを沈め、連動ギミックを起動
  (`self.MarkFinished`)
  (`PrimitiveComponent.SetMaterial` (`self.Button`) 0 "/Game/ChronoVault/Materials/Instances/MI_LampGreen.MI_LampGreen")
  (`GameplayStatics.PlaySoundAtLocation` "/Game/ChronoVault/Audio/SE/SE_Switch.SE_Switch" (`self.K2_GetActorLocation`) (struct) 1.0 1.0 0.0 null null null null)
  (`self.ActivateTargets`)
  (message `/Game/ChronoVault/Player/BPI_Player.PlayerShowMessage` GimmickInstigator (`self.PressedMessage`) 2.5)
  (bind (_direction _pressrate) (`Timeline|PressTimeline`)
    (:`Update`
      (`self.SetPressed` _pressrate))))

(event `self.OnRestore`
  ;[0.1 0.35 0.15 0.6] 復元：押された状態にする
  (`self.SetPressed` 1.0)
  (`PrimitiveComponent.SetMaterial` (`self.Button`) 0 "/Game/ChronoVault/Materials/Instances/MI_LampGreen.MI_LampGreen"))

(event `self.Trigger.OnComponentBeginOverlap`
  (params (OverlappedComponent :type "PrimitiveComponent Object Reference") (OtherActor :type "Actor Object Reference") (OtherComp :type "PrimitiveComponent Object Reference") (OtherBodyIndex :type Integer) (bFromSweep :type Boolean) (SweepResult :type "HitResult Structure (by ref)"))
  ;[0.4 0.25 0.05 0.6] プレイヤーが乗ったら作動
  (if (`KismetSystemLibrary.DoesImplementInterface` OtherActor "/Game/ChronoVault/Player/BPI_Player.BPI_Player_C")
    (message `/Game/ChronoVault/Gimmick/BPI_Gimmick.ActivateGimmick` self OtherActor)))

(fn `SetPressed`
  (params (Rate :type "Float (double-precision)"))
  ;[0.05 0.25 0.4 0.6] 押し込み量(0〜1)に応じてボタンを沈める
  (`SceneComponent.K2_SetRelativeLocation` (`self.Button`) (`KismetMathLibrary.VLerp` (0.0 0.0 16.0) (0.0 0.0 8.0) Rate) false false))

(fn `UserConstructionScript`
  (`parent.UserConstructionScript`))