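; Base Blueprint for ChronoVault gimmicks that trigger once and persist their finished state in BP_MyGameInstance under an EventName.
; BPI_Gimmick activation runs the child-overridden OnActivate only while unfinished; MarkFinished records completion.
; On BeginPlay, saved gimmicks are set finished and call OnRestore to restore state without effects.
; ActivateTargets chains activation to TargetGimmicks through the interface, passing itself as instigator.
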(event `OnActivate`
  (params (GimmickInstigator :type "Actor Object Reference"))
  ;[0.05 0.25 0.4 0.6] 作動時の処理（子BPでオーバーライド）
)

(event `OnRestore`
  ;[0.1 0.35 0.15 0.6] セーブ復元時の処理（子BPでオーバーライド）
)

(event `/Game/ChronoVault/Gimmick/BPI_Gimmick.ActivateGimmick`
  (params (GimmickInstigator :type "Actor Object Reference"))
  ;[0.4 0.25 0.05 0.6] BPI_Gimmick：未作動なら作動処理へ
  (if (not (`self.bFinished`))
    (`self.OnActivate` GimmickInstigator)))

(event `/Game/ChronoVault/Gimmick/BPI_Gimmick.SetEventFinished`
  ;[0.3 0.1 0.35 0.6] BPI_Gimmick：演出なしで作動済み状態にする
  (set `self.bFinished` true)
  (`self.OnRestore`))

(event `self.ReceiveBeginPlay`
  ;[0.4 0.08 0.1 0.6] 開始時：セーブ済みなら作動済み状態を復元
  (if (`/Game/ChronoVault/Core/BP_MyGameInstance.GetEventStatus` (cast `/Game/ChronoVault/Core/BP_MyGameInstance` (`GameplayStatics.GetGameInstance`) :!pure true) (`self.EventName`))
    (message `/Game/ChronoVault/Gimmick/BPI_Gimmick.SetEventFinished` self)))

(fn `ActivateTargets`
  ;[0.05 0.25 0.4 0.6] 連動先のギミックを BPI_Gimmick 経由で作動させる
  (for _array_element (`self.TargetGimmicks`)
    (message `/Game/ChronoVault/Gimmick/BPI_Gimmick.ActivateGimmick` _array_element self)))

(fn `MarkFinished`
  ;[0.05 0.25 0.4 0.6] 作動済みとして GameInstance に記録
  (set `self.bFinished` true)
  (`/Game/ChronoVault/Core/BP_MyGameInstance.SetEventStatus` (cast `/Game/ChronoVault/Core/BP_MyGameInstance` (`GameplayStatics.GetGameInstance`) :!pure true) (`self.EventName`) true))

(fn `UserConstructionScript`)