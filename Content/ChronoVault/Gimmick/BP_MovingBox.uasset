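; BP_MovingBox is a switch-linked gimmick box that moves between its origin and a relative EndOffset.
; On activation it calls MarkFinished to record its state, then StartMove; on restore it only calls StartMove to resume the motion.
; StartMove rebuilds the InterpToMovement control points from EndOffset, sets the duration from MoveTime and restarts the component.
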(event `self.OnActivate`
  (params (GimmickInstigator :type "Actor Object Reference"))
  ;[0.05 0.25 0.4 0.6] スイッチ連動：移動を開始し記録
  (`self.MarkFinished`)
  (`self.StartMove`))

(event `self.OnRestore`
  ;[0.1 0.35 0.15 0.6] 復元：移動を再開
  (`self.StartMove`))

(fn `StartMove`
  ;[0.05 0.25 0.4 0.6] InterpToMovement に往復の座標を設定して移動開始
  (set `InterpToMovementComponent.Duration` (`self.MoveTime`) (`self.InterpToMovement`))
  (`InterpToMovementComponent.ResetControlPoints` (`self.InterpToMovement`))
  (`InterpToMovementComponent.AddControlPointPosition` (`self.InterpToMovement`) (0.0 0.0 0.0) true)
  (`InterpToMovementComponent.AddControlPointPosition` (`self.InterpToMovement`) (`self.EndOffset`) true)
  (`InterpToMovementComponent.FinaliseControlPoints` (`self.InterpToMovement`))
  (`InterpToMovementComponent.RestartMovement` (`self.InterpToMovement`) 1.0)
  (`ActorComponent.Activate` (`self.InterpToMovement`) true))

(fn `UserConstructionScript`
  (`parent.UserConstructionScript`))