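; BP_Lever is a one-shot lever gimmick that the player pulls through the interact interface to trigger linked targets.
; Activation marks it finished, plays a switch sound, turns the grip lamp green, activates targets and shows the player a message.
; A timeline drives SetPulled to tilt the pivot, and restore snaps it straight to the pulled, green state.
; The interact prompt is blank once finished.
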(event `/Game/ChronoVault/Gimmick/BPI_Interact.Interact`
  (params (Interactor :type "Actor Object Reference"))
  ;[0.05 0.25 0.4 0.6] BPI_Interact：プレイヤーの操作で作動
  (message `/Game/ChronoVault/Gimmick/BPI_Gimmick.ActivateGimmick` self Interactor))

(event `self.OnActivate`
  (params (GimmickInstigator :type "Actor Object Reference"))
  ;[0.1 0.35 0.15 0.6] 作動：レバーを倒し、連動ギミックを起動
  (`self.MarkFinished`)
  (`GameplayStatics.PlaySoundAtLocation` "/Game/ChronoVault/Audio/SE/SE_Switch.SE_Switch" (`self.K2_GetActorLocation`) (struct) 1.0 1.0 0.0 null null null null)
  (`PrimitiveComponent.SetMaterial` (`self.Grip`) 0 "/Game/ChronoVault/Materials/Instances/MI_LampGreen.MI_LampGreen")
  (`self.ActivateTargets`)
  (message `/Game/ChronoVault/Player/BPI_Player.PlayerShowMessage` GimmickInstigator (`self.PulledMessage`) 2.5)
  (bind (_direction _pullrate) (`Timeline|LeverTimeline`)
    (:`Update`
      (`self.SetPulled` _pullrate))))

(event `self.OnRestore`
  ;[0.4 0.25 0.05 0.6] 復元：倒れた状態にする
  (`self.SetPulled` 1.0)
  (`PrimitiveComponent.SetMaterial` (`self.Grip`) 0 "/Game/ChronoVault/Materials/Instances/MI_LampGreen.MI_LampGreen"))

(fn `GetInteractText`
  (returns (InteractText :type Text))
  ;[0.05 0.25 0.4 0.6] 操作プロンプト（作動済みなら空＝非表示）
  (if (`self.bFinished`)
    (return "")
    (else
      (return "レバーを引く"))))

(fn `SetPulled`
  (params (Rate :type "Float (double-precision)"))
  ;[0.05 0.25 0.4 0.6] レバーの倒れ具合(0〜1)
  (`SceneComponent.K2_SetRelativeRotation` (`self.Pivot`) (`KismetMathLibrary.MakeRotator` 0.0 (`KismetMathLibrary.Lerp` 45.0 -45.0 Rate)) false false))

(fn `UserConstructionScript`
  (`parent.UserConstructionScript`))