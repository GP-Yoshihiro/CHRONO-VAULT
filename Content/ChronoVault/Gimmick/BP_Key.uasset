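; BP_Key is a collectible key, identified by KeyName, that a BPI_Player actor picks up by overlapping its trigger.
; Pickup passes the key to the player, records it in BP_MyGameInstance and destroys the actor, which also removes itself on BeginPlay if already taken.
; DT_KeyStatus supplies the display name and color for the pickup message and screen effect.
; The Construction Script applies that color to a dynamic material and the key's light.
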(event `self.ReceiveBeginPlay`
  ;[0.05 0.25 0.4 0.6] 開始時：取得済みの鍵なら消す
  (if (`/Game/ChronoVault/Core/BP_MyGameInstance.GetKeyStatus` (cast `/Game/ChronoVault/Core/BP_MyGameInstance` (`GameplayStatics.GetGameInstance`) :!pure true) (`self.KeyName`))
    (`self.K2_DestroyActor`)))

(event `self.Trigger.OnComponentBeginOverlap`
  (params (OverlappedComponent :type "PrimitiveComponent Object Reference") (OtherActor :type "Actor Object Reference") (OtherComp :type "PrimitiveComponent Object Reference") (OtherBodyIndex :type Integer) (bFromSweep :type Boolean) (SweepResult :type "HitResult Structure (by ref)"))
  ;[0.1 0.35 0.15 0.6] 接触で取得：BPI_Player へ渡し、取得状態を記録
  (if (`KismetSystemLibrary.DoesImplementInterface` OtherActor "/Game/ChronoVault/Player/BPI_Player.BPI_Player_C")
    (message `/Game/ChronoVault/Player/BPI_Player.PlayerAddItem` OtherActor (`self.KeyName`))
    (`/Game/ChronoVault/Core/BP_MyGameInstance.SetKeyStatus` (cast `/Game/ChronoVault/Core/BP_MyGameInstance` (`GameplayStatics.GetGameInstance`) :!pure true) (`self.KeyName`) true)
    (bind _returnvalue (`|GetDataTableRow` "/Game/ChronoVault/Data/DT_KeyStatus.DT_KeyStatus" (`self.KeyName`))
      (:`then`
        (bind (_displayname _description _keycolor) (break `/Game/ChronoVault/Data/S_KeyStatus` _returnvalue))
        (message `/Game/ChronoVault/Player/BPI_Player.PlayerShowMessage` OtherActor (`|FormatText` "{Name} を手に入れた" _displayname) 3.0)
        (message `/Game/ChronoVault/Player/BPI_Player.PlayerPlayScreenEffect` OtherActor _keycolor)
        (`GameplayStatics.PlaySound2D` "/Game/ChronoVault/Audio/SE/SE_Key.SE_Key" 1.0 1.0 0.0 null null))
      (:`RowNotFound`
        _))
    (`self.K2_DestroyActor`)))

(fn `UserConstructionScript`
  ;[0.05 0.25 0.4 0.6] DT_KeyStatus の色を鍵と光に反映
  (bind _returnvalue (`|GetDataTableRow` "/Game/ChronoVault/Data/DT_KeyStatus.DT_KeyStatus" (`self.KeyName`))
    (:`then`
      (bind _returnvalue_2 (`PrimitiveComponent.CreateDynamicMaterialInstance` (`self.KeyMesh`) 0 null "None"))
      (bind (_displayname _description _keycolor) (break `/Game/ChronoVault/Data/S_KeyStatus` _returnvalue))
      (`MaterialInstanceDynamic.SetVectorParameterValue` _returnvalue_2 "Color" _keycolor)
      (`LightComponent.SetLightColor` (`self.KeyLight`) _keycolor true))))