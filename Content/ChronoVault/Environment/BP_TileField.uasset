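; BP_TileField is an environment Blueprint that lays out copies of a single mesh in a flat grid.
; Its construction script clears the Tiles Instanced Static Mesh component, assigns TileMesh, then adds local-space instances across the X and Y counts and spacings.
; All tiles share one rotation and scale, and instancing keeps the rendering cost low.
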(fn `UserConstructionScript`
  ;[0.05 0.25 0.4 0.6] 同じメッシュを格子状に並べる（Instanced Static Meshで描画負荷を抑える）
  (`InstancedStaticMeshComponent.ClearInstances` (`self.Tiles`))
  (`StaticMeshComponent.SetStaticMesh` (`self.Tiles`) (`self.TileMesh`))
  (for _index (range (`self.CountX`))
    (for _index_2 (range (`self.CountY`))
      (`InstancedStaticMeshComponent.AddInstance` (`self.Tiles`) (`KismetMathLibrary.MakeTransform` (`KismetMathLibrary.MakeVector` (* (`KismetMathLibrary.Conv_IntToDouble` _index) (`self.SpacingX`)) (* (`KismetMathLibrary.Conv_IntToDouble` _index_2) (`self.SpacingY`))) (`self.TileRotation`) (`self.TileScale`)) false))))